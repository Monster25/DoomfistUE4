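; Player character with movement and four abilities: charged fist, slam, uppercut and an aerial-view teleport ultimate.
; Charged fist scales a forward launch and its duration by a timeline charge; uppercut launches up and forward, then briefly swaps gravity at the apex.
; Slam hops, then launches at a camera-trace hit, restoring input on landing.
; Ultimate pulls the spring arm out, then teleports to the camera-trace hit on Confirm or timeout.
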(event `InputAction|UltimateBoiii`
  (params (Key :type "Key Structure"))
  (bind _springarm (`self.SpringArm`))
  (bind (_returnvalue_roll _returnvalue_pitch _returnvalue_yaw) (`KismetMathLibrary.BreakRotator` (`SpringArmComponent.GetTargetRotation` (`self.SpringArm`))))
  ;[0 1 0.7573] Chad Thundercock Ult
  (:`Pressed`
    (set `self.bInUlt` true)
    (set `SpringArmComponent.TargetArmLength` (`self.UltVisionRange`) (`self.SpringArm`))
    (set `self.bCanMove` false)
    (set `self.bCanLook` false)
    (`KismetSystemLibrary.Delay` 1.0)
    (bind _returnvalue (`KismetSystemLibrary.K2_SetTimerDelegate` (delegate `FinishUlt`) (`self.TotalUltTime`)))
    (set `self.UltTimer` _returnvalue)
    (set `CharacterMovementComponent.MaxWalkSpeed` (`self.UltMovementSpeed`) (`self.CharacterMovement`))
    (set `SpringArmComponent.bInheritPitch` false _springarm)
    (`SceneComponent.K2_SetWorldRotation` _springarm (`KismetMathLibrary.MakeRotator` _returnvalue_roll (`self.UltCameraRotation`) _returnvalue_yaw) false false)
    (set `self.bCanMove` true)
    (set `self.bCanLook` true)))

(event `InputAction|ChargedFist`
  (params (Key :type "Key Structure"))
  ;[0.1792 1 0] Charged Fist
  (:`Pressed`
    (set `CharacterMovementComponent.MaxWalkSpeed` (`self.ChargeMovementSpeed`) (`self.CharacterMovement`))
    (`self.StartCharging`))
  (:`Released`
    (set `CharacterMovementComponent.MaxWalkSpeed` (`self.DefaultMovementSpeed`) (`self.CharacterMovement`))
    (`self.ReleaseFist`)))

(event `FinishUlt`
  (bind _springarm (`self.SpringArm`))
  (bind _camera (`self.Camera`))
  (bind (_ulthitlocation_x _ulthitlocation_y _ulthitlocation_z) (`KismetMathLibrary.BreakVector` (`self.UltHitLocation`)))
  (bind _returnvalue (`SceneComponent.K2_GetComponentLocation` _camera))
  ;[0 1 0.7573] Chad Thundercock Ult
  (bind (_outhit _returnvalue_2) (`KismetSystemLibrary.LineTraceSingle` :`Start` _returnvalue :`End` (+ _returnvalue (* (`SceneComponent.GetForwardVector` _camera) 9999999.0)) :`TraceChannel` "TraceTypeQuery1" :`DrawDebugType` "Persistent" :!label _label))
  (if _returnvalue_2
    (set `self.UltHitLocation` (`.Location` (`GameplayStatics.BreakHitResult` _outhit)))
    (set `self.bCanMove` false)
    (set `self.bCanLook` false)
    (`KismetSystemLibrary.Delay` 0.35)
    (set `CharacterMovementComponent.MaxWalkSpeed` (`self.DefaultMovementSpeed`) (`self.CharacterMovement`))
    (set `SpringArmComponent.bInheritPitch` true _springarm)
    (`SceneComponent.K2_SetWorldRotation` _springarm (`self.GetControlRotation`) false false)
    (set `SpringArmComponent.TargetArmLength` 0.0 (`self.SpringArm`))
    (`self.K2_SetActorLocation` (`KismetMathLibrary.MakeVector` _ulthitlocation_x _ulthitlocation_y (+ _ulthitlocation_z (`CapsuleComponent.CapsuleHalfHeight` (`self.CapsuleComponent`)))) false true)
    (set `self.bCanMove` true)
    (set `self.bCanLook` true)
    (set `self.bInUlt` false)))

(event `StartCharging`
  ;[0.1792 1 0] Charged Fist
  (bind (_direction _chargetime) (`Timeline|ChargeTimeline` :!via `PlayFromStart` :!label _label_2)
    (:`Update`
      (set `self.CurrentCharge` _chargetime))))

(event `InputAction|Confirm`
  (params (Key :type "Key Structure"))
  ;[0 1 0.7573] Chad Thundercock Ult
  (:`Pressed`
    (if (`self.bInUlt`)
      (`KismetSystemLibrary.K2_ClearAndInvalidateTimerHandle` (`self.UltTimer`))
      (goto _label))))

(event `ReleaseFist`
  (bind _charactermovement (`self.CharacterMovement`))
  (bind _charactermovement_2 (`self.CharacterMovement`))
  (bind _returnvalue (* (`self.FullChargeBoost`) (`self.CurrentCharge`)))
  ;[0.1792 1 0] Charged Fist
  (`|ExecutionSequence`
    (:`then_0`
      (goto _label_2 :!via `Stop`))
    (:`then_1`
      (set `self.bCanLook` false)
      (set `self.bCanMove` false)
      (set `CharacterMovementComponent.GravityScale` (`self.ChargedFistGravityScale`) _charactermovement)
      (set `CharacterMovementComponent.GroundFriction` (`self.FistGroundFriction`) _charactermovement)
      (`self.LaunchCharacter` (* (`self.GetActorForwardVector`) _returnvalue) true true)
      (`KismetSystemLibrary.Delay` (/ _returnvalue 8000.0))
      (set `CharacterMovementComponent.GravityScale` (`self.DefaultGravityScale`) _charactermovement_2)
      (set `CharacterMovementComponent.GroundFriction` (`self.DefaultGroundFriction`) _charactermovement_2)
      (set `self.bCanLook` true)
      (set `self.bCanMove` true)
      (set `MovementComponent.Velocity` (0.0 0.0 0.0) (`self.CharacterMovement`)))))

(event `InputAction|Jump`
  (params (Key :type "Key Structure"))
  ;[0.3091 0.3049 1] Movement
  (:`Pressed`
    (`self.Jump`))
  (:`Released`
    (`self.StopJumping`)))

(event `InputAxis|ForwardBackward`
  (params (AxisValue :type "Float (single-precision)"))
  ;[0.3091 0.3049 1] Movement
  (if (`self.bCanMove`)
    (`self.AddMovementInput` (`self.GetActorForwardVector`) AxisValue)))

(event `InputAction|Slam`
  (params (Key :type "Key Structure"))
  (bind _camera (`self.Camera`))
  (bind _returnvalue (`SceneComponent.K2_GetComponentLocation` _camera))
  ;[1 0.8613 0] Slam
  (:`Pressed`
    (bind (_outhit _returnvalue_2) (`KismetSystemLibrary.LineTraceSingle` :`Start` _returnvalue :`End` (+ _returnvalue (* (`SceneComponent.GetForwardVector` _camera) (`self.SlamRange`))) :`TraceChannel` "TraceTypeQuery1" :`DrawDebugType` "Persistent"))
    (if _returnvalue_2
      (set `self.bCanMove` false)
      (set `self.bCanLook` false)
      (set `self.SlamHitLocation` (`.Location` (`GameplayStatics.BreakHitResult` _outhit)))
      (`self.LaunchCharacter` (* (`self.GetActorUpVector`) (`self.SlamZUp`)) true true)
      (`KismetSystemLibrary.Delay` 0.2)
      (`self.LaunchCharacter` (* (`KismetMathLibrary.GetDirectionUnitVector` (`self.K2_GetActorLocation`) (`self.SlamHitLocation`)) (`self.SlamSpeed`)) true true))))

(event `InputAxis|LookLeftRight`
  (params (AxisValue :type "Float (single-precision)"))
  ;[0.3091 0.3049 1] Movement
  (if (`self.bCanLook`)
    (`self.AddControllerYawInput` AxisValue)))

(event `InputAxis|LeftRight`
  (params (AxisValue :type "Float (single-precision)"))
  ;[0.3091 0.3049 1] Movement
  (if (`self.bCanMove`)
    (`self.AddMovementInput` (`self.GetActorRightVector`) AxisValue)))

(event `InputAxis|LookUpDown`
  (params (AxisValue :type "Float (single-precision)"))
  ;[0.3091 0.3049 1] Movement
  (if (and (`self.bCanLook`) (`self.bCanLookUpDown`))
    (`self.AddControllerPitchInput` AxisValue)))

(event `self.OnLanded`
  (params (Hit :type "HitResult Structure (by ref)"))
  ;[1 0.8613 0] Slam
  (set `self.bCanMove` true)
  (set `self.bCanLook` true))

(event `InputAction|Uppercut`
  (params (Key :type "Key Structure"))
  (bind _charactermovement (`self.CharacterMovement`))
  (bind (_velocity_x _velocity_y) (`KismetMathLibrary.BreakVector` (`MovementComponent.Velocity` _charactermovement)))
  ;[1 0 0.9044] UPAHCAT
  (:`Pressed`
    (`self.LaunchCharacter` (+ (* (`self.GetActorUpVector`) (`self.UpPower`)) (* (`self.GetActorForwardVector`) (`self.ForwardPower`))) true true)
    (`KismetSystemLibrary.Delay` 0.25)
    (set `MovementComponent.Velocity` (`KismetMathLibrary.MakeVector` _velocity_x _velocity_y) _charactermovement)
    (set `CharacterMovementComponent.GravityScale` (`self.ApexGravityScale`) (`self.CharacterMovement`))
    (`KismetSystemLibrary.Delay` 0.5)
    (set `CharacterMovementComponent.GravityScale` (`self.DefaultGravityScale`) (`self.CharacterMovement`))))

(event `self.ReceiveBeginPlay`
  (bind _charactermovement (`self.CharacterMovement`))
  ;[1 0 0.07939] Save Defaults for Later ;)
  (set `self.DefaultGravityScale` (`CharacterMovementComponent.GravityScale` _charactermovement))
  (set `self.DefaultMovementSpeed` (`CharacterMovementComponent.MaxWalkSpeed` _charactermovement))
  (set `self.DefaultGroundFriction` (`CharacterMovementComponent.GroundFriction` (`self.CharacterMovement`)))
  (set `self.DefaultCameraRotation` (`SceneComponent.K2_GetComponentRotation` (`self.Camera`))))

(fn `UserConstructionScript`)